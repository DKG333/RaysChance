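; BP_Bullet is a projectile actor that damages enemies it overlaps, using a Box collision and ProjectileMovement.
; Box overlap casts the other actor to Bp_Enemy, passes Damage to EnemyDamageSystem and prints a debug message.
; A separate actor overlap checks for the "Enemy" tag, spawns an explosion effect at that actor's transform and destroys the bullet.
; Leftover BP_MasterPickUp ammo checks that would disable input are disconnected and never run.
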(event OnComponentDeactivated(ProjectileMovement)
  (params (Component :type Actor%20Component%20Object%20Reference)))

(event OnComponentBeginOverlap(Box)
  (params (OverlappedComponent :type Primitive%20Component%20Object%20Reference) (OtherActor :type Actor%20Object%20Reference) (OtherComp :type Primitive%20Component%20Object%20Reference) (OtherBodyIndex :type Integer) (bFromSweep :type Boolean) (SweepResult :type Hit%20Result%20Structure%20%28by%20ref%29))
  (bind _asbp_enemy (Utilities|Casting|CastToBp_Enemy OtherActor))
  (Default|EnemyDamageSystem _asbp_enemy (Variables|Default|Getdamage))
  (Development|PrintString "Hit enemy"))

(event EventBeginPlay)

(event Collision|EventActorBeginOverlap
  (params (OtherActor :type Actor%20Object%20Reference))
  (if (Actor|ActorHasTag OtherActor "Enemy")
    (Game|SpawnActorfromClass "/Game/StarterContent/Blueprints/Blueprint_Effect_Explosion.Blueprint_Effect_Explosion_C" (Transformation|GetActorTransform OtherActor) "Undefined" 0 0)
    (Actor|DestroyActor)))

(event EventTick
  (params (DeltaSeconds :type Float%20%28single-precision%29)))

(fn ConstructionScript)