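; AK47Ammo is an ammo pickup Blueprint that refills the player's AK47 when the Interaction input is pressed.
; If the AK47 reached through RayRef is valid and its MaxAmmo already equals PickUpAmmo, it prints a backpack-full message.
; Otherwise both comparison branches set MaxAmmo to PickUpAmmo rather than adding to it, then a pickup sound plays and the actor destroys itself.
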(event Input|ActionEvents|InputActionInteraction
  (params (Key :type Key%20Structure))
  (bind _rayref (Variables|Default|GetRayRef))
  (bind _rayref_2 (Variables|Default|GetRayRef))
  (bind _pickupammo (Variables|Default|GetPickUpAmmo))
  (bind _bpak47 (Variables|/Game/Player/Blueprints/Ray_bp/Ray_Bp.Ray_Bp_C|GetBPAK47 _rayref))
  (bind _bpak47_2 (Variables|/Game/Player/Blueprints/Ray_bp/Ray_Bp.Ray_Bp_C|GetBPAK47 _rayref_2))
  (bind _iteminfo (Variables|/Game/Player/Blueprints/Pickups_BP/BP_MasterPickUp.BP_MasterPickUp_C|GetItemInfo _bpak47_2))
  (bind _iteminfo_2 (Variables|/Game/Player/Blueprints/Pickups_BP/BP_MasterPickUp.BP_MasterPickUp_C|GetItemInfo _bpak47))
  (bind _maxammo (Utilities|Struct|BreakItem_Type _iteminfo))
  (:Pressed
    (if (Utilities|IsValid (Variables|/Game/Player/Blueprints/Ray_bp/Ray_Bp.Ray_Bp_C|GetBPAK47 (Variables|Default|GetRayRef)))
      (if (== _maxammo (Variables|Default|GetPickUpAmmo))
        (Development|PrintString "backpack fulll of ammo")
        (else
          (if (>= (+ (Variables|Default|GetPickUpAmmo) _maxammo) (Variables|Default|GetPickUpAmmo))
            (Utilities|Struct|SetmembersinItem_Type _iteminfo_2 _pickupammo)
            (else
              (Utilities|Struct|SetmembersinItem_Type _iteminfo_2 _pickupammo)))
          (Audio|PlaySound2D "/Game/Player/Sounds/216629__wiesenwiesel__picking-up-small-box-with-items-inside.216629__wiesenwiesel__picking-up-small-box-with-items-inside")
          (Actor|DestroyActor))))))

(fn ConstructionScript
  (|CallParentFunction))