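; Base ammo pickup actor that reacts when the Ray_Bp player character enters or leaves its sphere trigger.
; On overlap it stores the player reference, shows a prompt widget, outlines the mesh through custom depth and enables input from player controller 0.
; Leaving hides the widget and outline but does not disable input.
; The graph contains no ammo-granting or interaction logic.
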(event OnComponentBeginOverlap(Sphere1)
  (params (OverlappedComponent :type Primitive%20Component%20Object%20Reference) (OtherActor :type Actor%20Object%20Reference) (OtherComp :type Primitive%20Component%20Object%20Reference) (OtherBodyIndex :type Integer) (bFromSweep :type Boolean) (SweepResult :type Hit%20Result%20Structure%20%28by%20ref%29))
  (bind _asray_bp (Utilities|Casting|CastToRay_Bp OtherActor))
  (Variables|Default|SetRayRef _asray_bp)
  (Rendering|SetVisibility (Variables|Default|GetWidget) true false)
  (Rendering|SetRenderCustomDepth (Variables|Default|GetStaticMesh) true)
  (Input|EnableInput (Game|GetPlayerController 0)))

(event OnComponentEndOverlap(Sphere1)
  (params (OverlappedComponent :type Primitive%20Component%20Object%20Reference) (OtherActor :type Actor%20Object%20Reference) (OtherComp :type Primitive%20Component%20Object%20Reference) (OtherBodyIndex :type Integer))
  (bind _asray_bp (Utilities|Casting|CastToRay_Bp OtherActor))
  (Variables|Default|SetRayRef _asray_bp)
  (Rendering|SetVisibility (Variables|Default|GetWidget) false false)
  (Rendering|SetRenderCustomDepth (Variables|Default|GetStaticMesh) false))

(fn ConstructionScript)