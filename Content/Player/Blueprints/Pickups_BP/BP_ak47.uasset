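; BP_ak47 is an AK-47 weapon pickup that equips itself when an actor tagged "Player" overlaps it.
; On overlap it snaps to the "Weapon" socket on player 0's character mesh and turns off its own collision.
; It then casts that character to Ray_Bp and sets the held-weapon flags so AK47 is active and Pistol and NotHolding are cleared.
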(event EventBeginPlay)

(event Collision|EventActorBeginOverlap
  (params (OtherActor :type Actor%20Object%20Reference))
  (if (Actor|ActorHasTag OtherActor "Player")
    (Transformation|AttachComponentToComponent self (Variables|/Script/Engine.Character|GetMesh (Game|GetPlayerCharacter 0)) "Weapon" "SnapToTarget" "SnapToTarget" "SnapToTarget" true)
    (Collision|SetActorEnableCollision self false)
    (bind _asray_bp (Utilities|Casting|CastToRay_Bp (Game|GetPlayerCharacter 0)))
    (Variables|/Game/Player/Blueprints/Ray_bp/Ray_Bp.Ray_Bp_C|SetPistol _asray_bp false)
    (Variables|/Game/Player/Blueprints/Ray_bp/Ray_Bp.Ray_Bp_C|SetAK47 _asray_bp true)
    (Variables|/Game/Player/Blueprints/Ray_bp/Ray_Bp.Ray_Bp_C|SetNotHolding _asray_bp false)))

(event EventTick
  (params (DeltaSeconds :type Float%20%28single-precision%29)))

(fn ConstructionScript)