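; Base weapon pickup that the Ray_Bp player collects with Interaction when in range, highlighted by a widget and custom-depth outline.
; While firing, a Gate and retriggerable one-second delay loop camera line traces, applying random damage through the Damage_Bp interface.
; Item type selects the fire sound.
; The ItemInfo struct tracks ammo; manual or automatic reloads play a montage and refill the clip from reserves.
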(event OnComponentBeginOverlap(Sphere)
  (params (OverlappedComponent :type Primitive%20Component%20Object%20Reference) (OtherActor :type Actor%20Object%20Reference) (OtherComp :type Primitive%20Component%20Object%20Reference) (OtherBodyIndex :type Integer) (bFromSweep :type Boolean) (SweepResult :type Hit%20Result%20Structure%20%28by%20ref%29))
  (bind _asray_bp (Utilities|Casting|CastToRay_Bp OtherActor))
  (Variables|Default|SetRefrenceTopDownCharacter _asray_bp)
  (CallFunction|On/off true true)
  (Variables|Default|SetCanPick true)
  (Input|EnableInput (Game|GetPlayerController 0))
  (Physics|SetSimulatePhysics (Variables|Default|GetStaticMesh) false))

(event OnComponentEndOverlap(Sphere)
  (params (OverlappedComponent :type Primitive%20Component%20Object%20Reference) (OtherActor :type Actor%20Object%20Reference) (OtherComp :type Primitive%20Component%20Object%20Reference) (OtherBodyIndex :type Integer))
  (bind _asray_bp (Utilities|Casting|CastToRay_Bp OtherActor))
  (Variables|Default|SetRefrenceTopDownCharacter _asray_bp)
  (CallFunction|On/off false false)
  (Variables|Default|SetCanPick false))

(event Custom|Off/on
  (CallFunction|On/off false false)
  (Components|DestroyComponent (Variables|Default|GetSphere)))

(event Custom|StartFire
  (bind _refrencetopdowncharacter (Variables|Default|GetRefrenceTopDownCharacter))
  (bind _iteminfo (Variables|Default|GetItemInfo))
  (bind _itemtype (Utilities|Struct|BreakItem_Type _iteminfo))
  (bind _vr_camera (Variables|/Game/Player/Blueprints/Ray_bp/Ray_Bp.Ray_Bp_C|GetVR_Camera _refrencetopdowncharacter))
  (bind _returnvalue (Transformation|GetWorldLocation _vr_camera))
  (Utilities|FlowControl|Sequence
    (:then_0
      (goto _label Open))
    (:then_1
      (Utilities|FlowControl|Gate true :!label _label
        (:Exit
          (Utilities|FlowControl|Sequence
            (:then_0
              (Utilities|FlowControl|RetriggerableDelay 1.0)
              (goto _label))
            (:then_1
              (if (<= (.CurrentAmmo (Utilities|Struct|BreakItem_Type (Variables|Default|GetItemInfo))) 0)
                (Development|PrintString "out of ammo")
                (CallFunction|StoipFire)
                (else
                  (bind (_outhit _returnvalue_2) (Collision|LineTraceByChannel _returnvalue (+ _returnvalue (* (Math|Vector|GetForwardVector _vr_camera) 1e+03)) "TraceTypeQuery1" false 0 "None"))
                  (if _returnvalue_2
                    _
                    (else
                      _))
                  (Utilities|FlowControl|Sequence
                    (:then_0
                      (if (Utilities|Enum|Equal(Enum) _itemtype "NewEnumerator1")
                        (Audio|PlaySound2D "/Game/Player/Sounds/168707__qubodup__tank-firing.168707__qubodup__tank-firing")
                        (Animation|PlayAnimMontage (Variables|Default|GetRefrenceTopDownCharacter) (Variables|Default|GetPlayAnimFire) 1.0 "None" :!label _label_2)
                        (bind _structout (Utilities|Struct|SetmembersinItem_Type (Variables|Default|GetItemInfo) (- (.CurrentAmmo (Utilities|Struct|BreakItem_Type (Variables|Default|GetItemInfo))) 1)))
                        (if (Utilities|DoesObjectImplementInterface (.HitActor (Collision|BreakHitResult _outhit)) "/Game/Player/Blueprints/Damage_Bp.Damage_Bp_C")
                          (Class|DamageBp|TakeDamage(Message) (.HitActor (Collision|BreakHitResult _outhit)) (.HitBoneName (Collision|BreakHitResult _outhit)) (Math|Random|RandomFloatinRange 2e+01 35.0)))
                        (Effects|SpawnEmitteratLocation 0 (.Location (Collision|BreakHitResult _outhit)))))
                    (:then_1
                      (if (Utilities|Enum|Equal(Enum) _itemtype "NewEnumerator2")
                        (Audio|PlaySound2D "/Game/Player/Sounds/398597__cetsoundcrew__pistol-shot-ricochet.398597__cetsoundcrew__pistol-shot-ricochet")
                        (goto _label_2)))))))))))))

(event Custom|reLoad
  (bind _iteminfo (Variables|Default|GetItemInfo))
  (bind (_clipsize _currentammo) (Utilities|Struct|BreakItem_Type _iteminfo))
  ;[1 1 1] Reloading
  (if (== (Utilities|Struct|BreakItem_Type (Variables|Default|GetItemInfo)) 0)
    (Development|PrintString "find ammo")
    (elif (== _clipsize _currentammo)
      (Development|PrintString "full")
      (else
        (Variables|Default|SetIsReloading true)
        (if true
          (CallFunction|WeaponReload)
          (Utilities|FlowControl|Delay 2.0)
          (Variables|Default|SetIsReloading false))))))

(event Custom|FirePress
  ;[1 1 1] Reloading
  (Variables|Default|SetcanFire true)
  (if (not (Variables|Default|GetIsReloading))
    (CallFunction|StartFire)))

(event Custom|autoreload
  ;[1 1 1] Reloading
  (if (== (Utilities|Struct|BreakItem_Type (Variables|Default|GetItemInfo)) 0)
    (if (== (Utilities|Struct|BreakItem_Type (Variables|Default|GetItemInfo)) 0)
      (Development|PrintString "findammo")
      (else
        (Variables|Default|SetIsReloading true)
        (CallFunction|ReLoad)
        (Utilities|FlowControl|Delay 2.0)
        (Variables|Default|SetIsReloading false)))))

(event Custom|weaponReload
  (bind _iteminfo (Variables|Default|GetItemInfo))
  (bind _iteminfo_2 (Variables|Default|GetItemInfo))
  (bind _iteminfo_3 (Variables|Default|GetItemInfo))
  (bind _iteminfo_4 (Variables|Default|GetItemInfo))
  (bind (_currentammo _maxammo) (Utilities|Struct|BreakItem_Type _iteminfo_2))
  (bind (_clipsize _currentammo_2) (Utilities|Struct|BreakItem_Type _iteminfo_4))
  (bind _maxammo_2 (Utilities|Struct|BreakItem_Type _iteminfo))
  ;[1 1 1] Reloading
  (if (not (Variables|Default|GetcanFire))
    (Animation|PlayAnimMontage (Variables|Default|GetRefrenceTopDownCharacter) "/Game/Player/animations/Reloading_Montage.Reloading_Montage" 1.5 "None")
    (Audio|PlaySound2D "/Game/Player/Sounds/276959__gfl7__pistol-reload-sound.276959__gfl7__pistol-reload-sound")
    (if (> (Utilities|Struct|BreakItem_Type (Variables|Default|GetItemInfo)) 0)
      (Variables|Default|SetNeedsAmmo (- _clipsize _currentammo_2))
      (if (<= _maxammo_2 (Variables|Default|GetNeedsAmmo))
        (Utilities|Struct|SetmembersinItem_Type _iteminfo_3 (+ _currentammo _maxammo))
        (Utilities|Struct|SetmembersinItem_Type _iteminfo_3)
        (else
          (Utilities|Struct|SetmembersinItem_Type _iteminfo_3 (- _maxammo_2 (Variables|Default|GetNeedsAmmo)))
          (Utilities|Struct|SetmembersinItem_Type _iteminfo_3 (Utilities|Struct|BreakItem_Type (Variables|Default|GetItemInfo))))))))

(event Custom|StoipFire
  (bind _refrencetopdowncharacter (Variables|Default|GetRefrenceTopDownCharacter))
  (bind _iteminfo (Variables|Default|GetItemInfo))
  (bind _itemtype (Utilities|Struct|BreakItem_Type _iteminfo))
  (bind _vr_camera (Variables|/Game/Player/Blueprints/Ray_bp/Ray_Bp.Ray_Bp_C|GetVR_Camera _refrencetopdowncharacter))
  (bind _returnvalue (Transformation|GetWorldLocation _vr_camera))
  (Utilities|FlowControl|Gate true) ; enters at Close
)

(event Custom|fireRelease
  ;[1 1 1] Reloading
  (Variables|Default|SetcanFire false)
  (CallFunction|StoipFire)
  (CallFunction|Autoreload))

(event Input|ActionEvents|InputActionInteraction
  (params (Key :type Key%20Structure))
  (:Pressed
    (if (Variables|Default|GetCanPick)
      (Default|PickUp (Variables|Default|GetRefrenceTopDownCharacter) self))))

(fn ConstructionScript
  (Variables|Default|SetItemInfo (Utilities|Struct|MakeItem_Type (.itemtype (Variables|Default|GetItemInfo)) (Utilities|GetClass self) (.clipsize (Variables|Default|GetItemInfo)) (.currentammo (Variables|Default|GetItemInfo)) (.maxammo (Variables|Default|GetItemInfo)) (.damage (Variables|Default|GetItemInfo)) (.itemimage (Variables|Default|GetItemInfo)) (.equipsocketname (Variables|Default|GetItemInfo)) (.unequipnamesocket (Variables|Default|GetItemInfo)))))

(fn On/off
  (params (bNewVisibility :type Boolean) (bValue :type Boolean))
  (Rendering|SetVisibility (Variables|Default|GetWidget) bNewVisibility false)
  (Rendering|SetRenderCustomDepth (Variables|Default|GetStaticMesh) bValue))