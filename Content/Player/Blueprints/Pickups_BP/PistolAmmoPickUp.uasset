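; Pistol ammo pickup Blueprint that refills the player's pistol reserve when the Interaction input is pressed.
; It reaches the pistol through RayRef and, if MaxAmmo already equals PickUpAmmo, prints a backpack-full message.
; Otherwise both comparison branches set MaxAmmo to PickUpAmmo rather than adding to it, then it plays a 2D sound and destroys itself.
; The input handler checks only that the pistol reference is valid, with no range or focus test.
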(event Input|ActionEvents|InputActionInteraction
  (params (Key :type Key%20Structure))
  (bind _rayref (Variables|Default|GetRayRef))
  (bind _rayref_2 (Variables|Default|GetRayRef))
  (bind _pickupammo (Variables|Default|GetPickUpAmmo))
  (bind _pistolbp (Variables|/Game/Player/Blueprints/Ray_bp/Ray_Bp.Ray_Bp_C|GetPistolBp _rayref))
  (bind _pistolbp_2 (Variables|/Game/Player/Blueprints/Ray_bp/Ray_Bp.Ray_Bp_C|GetPistolBp _rayref_2))
  (bind _iteminfo (Variables|/Game/Player/Blueprints/Pickups_BP/BP_MasterPickUp.BP_MasterPickUp_C|GetItemInfo _pistolbp_2))
  (bind _iteminfo_2 (Variables|/Game/Player/Blueprints/Pickups_BP/BP_MasterPickUp.BP_MasterPickUp_C|GetItemInfo _pistolbp))
  (bind _maxammo (Utilities|Struct|BreakItem_Type _iteminfo))
  (:Pressed
    (if (Utilities|IsValid (Variables|/Game/Player/Blueprints/Ray_bp/Ray_Bp.Ray_Bp_C|GetPistolBp (Variables|Default|GetRayRef)))
      (if (== _maxammo (Variables|Default|GetPickUpAmmo))
        (Development|PrintString "backpack fulll of ammo")
        (else
          (if (>= (+ (Variables|Default|GetPickUpAmmo) _maxammo) (Variables|Default|GetPickUpAmmo))
            (Utilities|Struct|SetmembersinItem_Type _iteminfo_2 _pickupammo)
            (else
              (Utilities|Struct|SetmembersinItem_Type _iteminfo_2 _pickupammo)))
          (Audio|PlaySound2D 0)
          (Actor|DestroyActor))))))

(fn ConstructionScript
  (|CallParentFunction))