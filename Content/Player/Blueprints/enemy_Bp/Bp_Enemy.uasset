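; Enemy pawn that chases the Ray_Bp player character and damages it on contact.
; PawnSensing starts an AI MoveTo toward the seen player, and a box overlap calls the player's DamageSystem.
; EnemyDamageSystem subtracts health, then at zero plays a death montage and destroys the actor after a short delay.
; Game-over, level-load and explosion nodes are disconnected, and DirectionSpawn holds only an unused transform.
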(event OnSeePawn(PawnSensing)
  (params (Pawn :type Pawn%20Object%20Reference))
  (bind _asray_bp (Utilities|Casting|CastToRay_Bp Pawn))
  (AI|AIMoveTo self "0, 0, 0" _asray_bp 5.0 false))

(event OnComponentBeginOverlap(Box1)
  (params (OverlappedComponent :type Primitive%20Component%20Object%20Reference) (OtherActor :type Actor%20Object%20Reference) (OtherComp :type Primitive%20Component%20Object%20Reference) (OtherBodyIndex :type Integer) (bFromSweep :type Boolean) (SweepResult :type Hit%20Result%20Structure%20%28by%20ref%29))
  (bind _asray_bp (Utilities|Casting|CastToRay_Bp OtherActor))
  (Default|DamageSystem _asray_bp (Variables|Default|GetDamage)))

(event Custom|EnemyDamageSystem
  (params (Damage%20in :type Float%20%28single-precision%29))
  ;[1 1 1] killing the enemy
  (Variables|Default|SetisHit true)
  (bind _output_get (Variables|Default|SetEnemyHealth (- (Variables|Default|GetEnemyHealth) Damage%20in)))
  (Development|PrintString (Utilities|String|ToString(Float) (Variables|Default|GetEnemyHealth)))
  (if (<= _output_get 0.0)
    (Animation|PlayAnimMontage "/Game/Player/animations/Dying_Backwards_Montage.Dying_Backwards_Montage" 2.0 "None")
    (Input|DisableInput (Game|GetPlayerController 0))
    (Variables|Default|SetIsDead true)
    (Utilities|FlowControl|Delay 0.5)
    (Actor|DestroyActor)))

(event EventTick
  (params (DeltaSeconds :type Float%20%28single-precision%29)))

(fn ConstructionScript)