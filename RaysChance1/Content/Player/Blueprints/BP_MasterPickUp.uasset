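; BP_MasterPickUp is a pickup weapon base that Ray_Bp characters collect and use to fire and reload.
; Sphere overlap toggles a widget and custom-depth highlight, letting the Interaction input pass the item to the character's PickUp.
; Fire press and release start and stop firing, with release triggering an auto-reload check on empty clips.
; Reloading plays a character montage, refills the ItemInfo clip from reserve ammo and uses two-second delays to clear IsReloading.
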(event OnComponentBeginOverlap(Sphere)
  (params (OverlappedComponent :type Primitive%20Component%20Object%20Reference) (OtherActor :type Actor%20Object%20Reference) (OtherComp :type Primitive%20Component%20Object%20Reference) (OtherBodyIndex :type Integer) (bFromSweep :type Boolean) (SweepResult :type Hit%20Result%20Structure%20%28by%20ref%29))
  (bind _asray_bp (Utilities|Casting|CastToRay_Bp OtherActor))
  (Variables|Default|SetRefrenceTopDownCharacter _asray_bp)
  (CallFunction|On/off true true)
  (Variables|Default|SetCanPick true)
  (Input|EnableInput (Game|GetPlayerController 0)))

(event OnComponentEndOverlap(Sphere)
  (params (OverlappedComponent :type Primitive%20Component%20Object%20Reference) (OtherActor :type Actor%20Object%20Reference) (OtherComp :type Primitive%20Component%20Object%20Reference) (OtherBodyIndex :type Integer))
  (bind _asray_bp (Utilities|Casting|CastToRay_Bp OtherActor))
  (Variables|Default|SetRefrenceTopDownCharacter _asray_bp)
  (CallFunction|On/off false false)
  (Variables|Default|SetCanPick false))

(event Custom|Off/on
  (CallFunction|On/off false false)
  (Components|DestroyComponent (Variables|Default|GetSphere)))

(event Custom|reLoad
  (bind _iteminfo (Variables|Default|GetItemInfo))
  (bind (_clipsize _currentammo _clipsize_2) (Utilities|Struct|BreakItem_Type _iteminfo))
  (if (== (.MaxAmmo (Utilities|Struct|BreakItem_Type (Variables|Default|GetItemInfo))) 0)
    (Development|PrintString "find ammo")
    (elif (== _clipsize_2 _currentammo)
      (Development|PrintString "full")
      (else
        (bind _output_get (Variables|Default|SetIsReloading true))
        (if _output_get
          (CallFunction|WeaponReload)
          (Utilities|FlowControl|Delay 2.0)
          (Variables|Default|SetIsReloading false))))))

(event Custom|FirePress
  (Variables|Default|SetcanFire true)
  (if (not (Variables|Default|GetIsReloading))
    (CallFunction|StartFire)))

(event Custom|autoreload
  (if (== (.CurrentAmmo (Utilities|Struct|BreakItem_Type (Variables|Default|GetItemInfo))) 0)
    (if (== (.MaxAmmo (Utilities|Struct|BreakItem_Type (Variables|Default|GetItemInfo))) 0)
      (Development|PrintString "fireammo")
      (else
        (Variables|Default|SetIsReloading true)
        (CallFunction|ReLoad)
        (Utilities|FlowControl|Delay 2.0)
        (Variables|Default|SetIsReloading false)))))

(event Custom|weaponReload
  (bind _iteminfo (Variables|Default|GetItemInfo))
  (bind _iteminfo_2 (Variables|Default|GetItemInfo))
  (bind _iteminfo_3 (Variables|Default|GetItemInfo))
  (bind _iteminfo_4 (Variables|Default|GetItemInfo))
  (bind (_clipsize _currentammo _maxammo) (Utilities|Struct|BreakItem_Type _iteminfo_2))
  (bind (_clipsize_2 _currentammo_2) (Utilities|Struct|BreakItem_Type _iteminfo_4))
  (bind _maxammo_2 (Utilities|Struct|BreakItem_Type _iteminfo))
  (if (not (Variables|Default|GetcanFire))
    (Animation|PlayAnimMontage (Variables|Default|GetRefrenceTopDownCharacter) 0 1.5 "None")
    (if (> (.MaxAmmo (Utilities|Struct|BreakItem_Type (Variables|Default|GetItemInfo))) 0)
      (Variables|Default|SetNeedsAmmo (- _clipsize_2 _currentammo_2))
      (if (<= _maxammo_2 (Variables|Default|GetNeedsAmmo))
        (Utilities|Struct|SetmembersinItem_Type _iteminfo_3 (+ _currentammo _maxammo))
        (Utilities|Struct|SetmembersinItem_Type _iteminfo_3)
        (else
          (Utilities|Struct|SetmembersinItem_Type _iteminfo_3 (- _maxammo_2 (Variables|Default|GetNeedsAmmo)))
          (Utilities|Struct|SetmembersinItem_Type _iteminfo_3 (Utilities|Struct|BreakItem_Type (Variables|Default|GetItemInfo))))))))

(event Custom|fireRelease
  (Variables|Default|SetcanFire false)
  (CallFunction|StoipFire)
  (CallFunction|Autoreload))

(event Input|ActionEvents|InputActionInteraction
  (params (Key :type Key%20Structure))
  (:Pressed
    (if (Variables|Default|GetCanPick)
      (Default|PickUp (Variables|Default|GetRefrenceTopDownCharacter) self))))

(fn ConstructionScript
  (Variables|Default|SetItemInfo (Utilities|Struct|MakeItem_Type (.itemtype (Variables|Default|GetItemInfo)) (Utilities|GetClass self) 0 (.currentammo (Variables|Default|GetItemInfo)) (.maxammo (Variables|Default|GetItemInfo)) (.damage (Variables|Default|GetItemInfo)) (.itemimage (Variables|Default|GetItemInfo)) (.equipsocketname (Variables|Default|GetItemInfo)) (.unequipnamesocket (Variables|Default|GetItemInfo)))))

(fn On/off
  (params (bNewVisibility :type Boolean) (bValue :type Boolean))
  (Rendering|SetVisibility (Variables|Default|GetWidget) bNewVisibility false)
  (Rendering|SetRenderCustomDepth (Variables|Default|GetStaticMesh) bValue))